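; BP_Force is a spline actor that lines its path with repeated static mesh components.
; The construction script derives a segment count from spline length at a fixed spacing, then adds a mesh at each step, endpoints included.
; Each mesh takes its local location and rotation from constant-velocity sampling, so spacing stays even along the curve.
; The event graph holds only disabled placeholder events, with no runtime logic.
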(fn `UserConstructionScript`
  (bind _spline (`self.Spline`))
  (bind _returnvalue (`KismetMathLibrary.FTrunc` (/ (`SplineComponent.GetSplineLength` _spline) 150.0)))
  (for _index (range (+ _returnvalue 1))
    (bind _returnvalue_2 (* (`KismetMathLibrary.Conv_IntToDouble` _index) (/ 1.0 (`KismetMathLibrary.Conv_IntToDouble` _returnvalue))))
    (`AddComponent|NODE_AddStaticMeshComponent-0` :`RelativeTransform` (`KismetMathLibrary.MakeTransform` (`SplineComponent.GetLocationAtTime` _spline _returnvalue_2 "Local" true) (`SplineComponent.GetRotationAtTime` _spline _returnvalue_2 "Local" true)))))